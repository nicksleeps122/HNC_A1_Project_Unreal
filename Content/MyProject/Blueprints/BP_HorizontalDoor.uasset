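; BP_HorizontalDoor is a door that slides along Y when a BP_SideScrollingCharacter begins or ends overlapping it, unless Locked is set.
; Each overlap event restarts its own Timeline, one for entering and one for leaving.
; Each Timeline update feeds its track value as a DeltaY into MoveUpdatedComponent on InterpToMovement, so movement is applied as per-update offsets.
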(event `self.ReceiveActorBeginOverlap`
  (params (OtherActor :type "Actor Object Reference"))
  (if (not (`self.Locked`))
    (cast `/Game/Variant_SideScroller/Blueprints/BP_SideScrollingCharacter` OtherActor)
    (bind (_direction _doormovement) (`Timeline|Timeline` :!via `PlayFromStart`)
      (:`Update`
        (`MovementComponent.K2_MoveUpdatedComponent` :`self` (`self.InterpToMovement`) :`Delta` (`KismetMathLibrary.MakeVector` 0.0 _doormovement))))))

(event `self.ReceiveActorEndOverlap`
  (params (OtherActor :type "Actor Object Reference"))
  (if (not (`self.Locked`))
    (cast `/Game/Variant_SideScroller/Blueprints/BP_SideScrollingCharacter` OtherActor)
    (bind (_direction _newtrack_0) (`Timeline|Timeline_0` :!via `PlayFromStart`)
      (:`Update`
        (`MovementComponent.K2_MoveUpdatedComponent` :`self` (`self.InterpToMovement`) :`Delta` (`KismetMathLibrary.MakeVector` 0.0 _newtrack_0))))))

(fn `UserConstructionScript`)