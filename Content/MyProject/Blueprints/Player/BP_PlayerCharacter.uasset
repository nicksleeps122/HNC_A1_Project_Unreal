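; BP_PlayerCharacter is a 2D Paper flipbook player character with move, jump and dash input.
; Move and dash feed movement input along world X, with dash using a fixed larger scale.
; Tick consumes that input and offsets the capsule directly, without sweep or delta-time scaling.
; The flipbook starts frozen; move input toggles its play rate and rewinds it after a short delay, while Interact is empty.
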(event `self.ReceiveTick`
  (params (DeltaSeconds :type "Float (single-precision)"))
  (bind _returnvalue (`self.ConsumeMovementInputVector`))
  (`SceneComponent.K2_AddRelativeLocation` (`self.CapsuleComponent`) _returnvalue false false))

(event `self.ReceiveBeginPlay`
  (`PaperFlipbookComponent.SetPlayRate` (`self.PaperFlipbook`) 0.0))

(event `EnhancedInput|/Game/MyProject/Blueprints/Player/IA_PlatformingInteract`
  (params (ActionValue :type Boolean) (ElapsedSeconds :type "Float (double-precision)") (TriggeredSeconds :type "Float (double-precision)") (InputAction :type "InputAction Object Reference" :default "/Game/MyProject/Blueprints/Player/IA_PlatformingInteract.IA_PlatformingInteract")))

(event `EnhancedInput|/Game/MyProject/Blueprints/Player/IA_PlatformingMove`
  (params (ActionValue :type "Float (double-precision)") (ElapsedSeconds :type "Float (double-precision)") (TriggeredSeconds :type "Float (double-precision)") (InputAction :type "InputAction Object Reference" :default "/Game/MyProject/Blueprints/Player/IA_PlatformingMove.IA_PlatformingMove"))
  (bind _paperflipbook (`self.PaperFlipbook`))
  (:`Triggered`
    (`PaperFlipbookComponent.SetPlayRate` _paperflipbook 1.0)
    (`self.AddMovementInput` (1.0 0.0 0.0) ActionValue)
    (`PaperFlipbookComponent.SetPlayRate` _paperflipbook 0.0)
    (`KismetSystemLibrary.Delay` 0.2)
    (`PaperFlipbookComponent.SetPlaybackPosition` _paperflipbook 0.0 false)))

(event `EnhancedInput|/Game/MyProject/Blueprints/Player/IA_PlatformingJump`
  (params (ActionValue :type Boolean) (ElapsedSeconds :type "Float (double-precision)") (TriggeredSeconds :type "Float (double-precision)") (InputAction :type "InputAction Object Reference" :default "/Game/MyProject/Blueprints/Player/IA_PlatformingJump.IA_PlatformingJump"))
  (:`Triggered`
    (`self.Jump`)))

(event `EnhancedInput|/Game/MyProject/Blueprints/Player/IA_PlatformingDash`
  (params (ActionValue :type Boolean) (ElapsedSeconds :type "Float (double-precision)") (TriggeredSeconds :type "Float (double-precision)") (InputAction :type "InputAction Object Reference" :default "/Game/MyProject/Blueprints/Player/IA_PlatformingDash.IA_PlatformingDash"))
  (:`Triggered`
    (`self.AddMovementInput` (1.0 0.0 0.0) 3.0)))

(fn `UserConstructionScript`)